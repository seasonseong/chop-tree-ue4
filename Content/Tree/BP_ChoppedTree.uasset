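; BP_ChoppedTree is the chopped counterpart of BP_Tree, taking on the state of the tree that owns it.
; On BeginPlay it casts its owner to BP_Tree and copies the chop map texture, chop map length and tree info, then calls UpdateMaterialParameters to apply them.
; If the owner is not a BP_Tree, neither the copy nor the material update runs.
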(event EventBeginPlay
  (|CallParentFunction)
  ;[1 0.1172 0] ChopMapTexture, TreeInfo, ChopMapLength 등 나무의 정보를 복사합니다
  (bind _asbp_tree (Utilities|Casting|CastToBP_Tree (Components|GetOwner)))
  (Utilities|FlowControl|Sequence
    (:then_0
      (Variables|Default|SetChopMapTexture (Variables|/Game/Tree/BP_Tree.BP_Tree_C|GetChopMapTexture _asbp_tree))
      (Variables|Default|SetTreeInfo (Variables|/Game/Tree/BP_Tree.BP_Tree_C|GetTreeInfo _asbp_tree))
      (Variables|Default|SetChopMapLength (Variables|/Game/Tree/BP_Tree.BP_Tree_C|GetChopMapLength _asbp_tree)))
    (:then_1
      (CallFunction|Update(MaterialParameters)))))

(fn ConstructionScript
  (|CallParentFunction))