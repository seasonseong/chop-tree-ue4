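; Tree actor Blueprint that prepares a choppable trunk, with chop damage mapped by angle around a chop plane.
; Construction creates a render-target ChopMap texture and dynamic MI_Tree material, passes it chop dimensions and the plane's local-space axes, then resets the ChopMap array.
; Helpers provide signed angles, wrap-around index distance and linear damage falloff across the hit arc.
; No graph here applies damage or draws to the texture.
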(event EventBeginPlay
  (|CallParentFunction))

(event Collision|EventActorBeginOverlap
  (params (OtherActor :type Actor%20Object%20Reference)))

(event EventTick
  (params (DeltaSeconds :type Float%20%28single-precision%29)))

(fn ConstructionScript
  (|CallParentFunction)
  (Initialize|Initialize(Variables))
  (Update|Update(MaterialParameters))
  (Clear|Clear(Variables)))

(fn GetSignedDegreeBetweenVectors
  (params (A :type Vector) (B :type Vector) (PositiveAxis :type Vector))
  (return (* (select (>= (Math|Vector|DotProduct (Math|Vector|CrossProduct A B) PositiveAxis) 0.0) 1.0 -1.0) (Math|Float|Absolute(Float) (Class|KismetMathLibrary|DegAcos (Math|Vector|DotProduct A B))))))

(fn ClampIndex
  (params (Index :type Integer))
  (LocalVariables|SetModulaIndex (Math|Integer|%(Integer) Index (Variables|Data|GetChopMapLength)))
  (if (< (LocalVariables|GetModulaIndex) 0) ; 음수면
    (return (|({2D9795EA-4B89-6AA1-F70C-53B277E84997}+{EBCEE680-45A4-6C14-DFBA-FF9408E3DA09})))
    (else
      (return (LocalVariables|GetModulaIndex)))))

(fn Initialize(Variables)
  (Utilities|FlowControl|Sequence
    (:then_0
      (bind _returnvalue (Rendering|CreateRenderTarget2D (Variables|Data|GetChopMapLength) 2 "RTF_RGBA16f"))
      (Variables|Runtime|SetChopMapTexture _returnvalue))
    (:then_1
      (bind _returnvalue_2 (Rendering|Material|CreateDynamicMaterialInstance "/Game/Tree/Material/MI_Tree.MI_Tree" "None" "None" :!class /Script/Engine.KismetMaterialLibrary))
      (bind _output_get (Variables|Runtime|SetTreeDMI _returnvalue_2))
      (Rendering|Material|SetMaterial (Variables|Debug|GetStaticMeshComponent) 0 _output_get))))

(fn Update(MaterialParameters)
  (Rendering|Material|SetTextureParameterValue (Variables|Runtime|GetTreeDMI) "ChopMapTexture" (Variables|Runtime|GetChopMapTexture)) ; 호출하기전에 TreeDMI와 ChopMapTexture가 제대로 초기화되었는지 확인해주세요
  (Rendering|Material|SetScalarParameterValue (Variables|Runtime|GetTreeDMI) "ChopDepth" (Utilities|Struct|BreakF_TreeInfo (Variables|Data|GetTreeInfo)) :!class /Script/Engine.MaterialInstanceDynamic)
  (Rendering|Material|SetScalarParameterValue (Variables|Runtime|GetTreeDMI) "ChopHalfHeight" (Utilities|Struct|BreakF_TreeInfo (Variables|Data|GetTreeInfo)) :!class /Script/Engine.MaterialInstanceDynamic)
  (Rendering|Material|SetScalarParameterValue (Variables|Runtime|GetTreeDMI) "ChopMapLength" (Math|Conversions|ToFloat(Integer) (Variables|Data|GetChopMapLength)) :!class /Script/Engine.MaterialInstanceDynamic)
  (Rendering|Material|SetVectorParameterValue (Variables|Runtime|GetTreeDMI) "ChopPlane_Origin_Local" (Utility|VectortoLinearColor (Variables|/Script/Engine.SceneComponent|GetRelativeLocation (Variables|Data|GetChopPlane))) :!class /Script/Engine.MaterialInstanceDynamic)
  (Rendering|Material|SetVectorParameterValue (Variables|Runtime|GetTreeDMI) "ChopPlane_Normal_Local" (Utility|VectortoLinearColor (Utility|ToRelativeNormal (Math|Vector|GetUpVector (Variables|Data|GetChopPlane)))) :!class /Script/Engine.MaterialInstanceDynamic)
  (Rendering|Material|SetVectorParameterValue (Variables|Runtime|GetTreeDMI) "ChopPlane_Forward_Local" (Utility|VectortoLinearColor (Utility|ToRelativeNormal (Math|Vector|GetForwardVector (Variables|Data|GetChopPlane)))) :!class /Script/Engine.MaterialInstanceDynamic))

(fn VectortoLinearColor
  (params (Vector :type Vector))
  (bind (_x _y _z) (Math|Vector|BreakVector Vector))
  (return (Math|Color|MakeColor _x _y _z)))

(fn Clear(Variables)
  (Utilities|Array|Clear (Variables|Runtime|GetChopMap))
  (Utilities|Array|Resize (Variables|Runtime|GetChopMap) (Variables|Data|GetChopMapLength)))

(fn AffectedIndicesRange
  (return (* (Math|Conversions|ToFloat(Integer) (Variables|Data|GetChopMapLength)) (/ (Variables|Data|External|GetHitAngle) 3.6e+02))))

(fn GetAttanuatedDamage
  (params (CenterIndex :type Integer) (MyIndex :type Integer) (BaseDamage :type Float%20%28single-precision%29))
  (return (* (- 1.0 (/ (Math|Conversions|ToFloat(Integer) (Math|Integer|Absolute(Integer) (Utility|DistanceBetweenIndices CenterIndex MyIndex))) (* (Utility|AffectedIndicesRange) 0.5))) BaseDamage)))

(fn DistanceBetweenIndices
  (params (A :type Integer) (B :type Integer))
  (LocalVariables|SetClampedA (Utility|ClampIndex A))
  (LocalVariables|SetClampedB (Utility|ClampIndex B))
  (return (.MinValue (Math|Integer|MinOfIntArray (Utilities|Array|MakeArray (|(abs(({AFAA21D7-4B98-D2A9-7074-019418A761DC}-{A56C19A8-4826-B667-5B59-A79439EE9052})))) (|(abs((({AFAA21D7-4B98-D2A9-7074-019418A761DC}+{EBCEE680-45A4-6C14-DFBA-FF9408E3DA09})-{A56C19A8-4826-B667-5B59-A79439EE9052})))) (|(abs(({A56C19A8-4826-B667-5B59-A79439EE9052}-{AFAA21D7-4B98-D2A9-7074-019418A761DC})))) (|(abs((({A56C19A8-4826-B667-5B59-A79439EE9052}+{EBCEE680-45A4-6C14-DFBA-FF9408E3DA09})-{AFAA21D7-4B98-D2A9-7074-019418A761DC})))))))))

(fn ToRelativeNormal
  (params (InVec :type Vector))
  (return (Math|Vector|Normalize (Math|Rotator|GetRotationXVector (Math|Transform|InverseTransformRotation (Transformation|GetActorTransform) (Math|Conversions|RotationFromXVector InVec))))))