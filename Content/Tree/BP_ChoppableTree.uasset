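; Choppable tree actor that accumulates damage around its trunk and falls once chopped enough.
; Chop projects each hit onto ChopPlane, maps its signed angle to a ChopMap index, and adds attenuated damage to neighboring entries.
; The array is drawn into the ChopMapTexture render target as a one-pixel-high grayscale strip.
; Once about a quarter is saturated, the next chop swaps in the stump and spawns BP_ChoppedTree, toppled by impulse away from the hit.
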(fn ConstructionScript
  (|CallParentFunction)
  (Utilities|FlowControl|Sequence
    (:then_0
      (Initialize|Initialize(BottomStaticMesh)))
    (:then_1
      ;[0.7813 0 1] 잘리지 않은 온전한 모습을 보여야하므로 나무 밑동을 숨깁니다
      (Update|Update(BottomStaticMesh) false)
      (Update|Update(MainStaticMesh) true))))

(fn Chop
  (params (HitResult :type Hit%20Result%20Structure))
  (bind _returnvalue (CallFunction|AffectedIndicesRange))
  (bind _returnvalue_2 (/ _returnvalue 2.0))
  (bind _returnvalue_3 (Math|Float|Round _returnvalue_2))
  (LocalVariables|SetHitPoint (.ImpactPoint (Collision|BreakHitResult HitResult)))
  (Utilities|FlowControl|Sequence
    (:then_0
      (LocalVariables|SetProjectedHitPoint (Class|KismetMathLibrary|ProjectPointontoPlane (LocalVariables|GetHitPoint) (Transformation|GetWorldLocation (Variables|Default|GetChopPlane)) (Math|Vector|GetUpVector (Variables|Default|GetChopPlane))))
      (LocalVariables|SetToProjectedHitPoint (Math|Vector|Normalize (- (LocalVariables|GetProjectedHitPoint) (Transformation|GetWorldLocation (Variables|Default|GetChopPlane))))))
    (:then_1
      (if (Utility|IsChoppedEnough)
        (Update|Update(MainStaticMesh) false)
        (Update|Update(BottomStaticMesh) true)
        ;[0 1 0.3906] 첫 한 번만 태우도록
        (if (not (Variables|Default|GetIsChopped))
          (Variables|Default|SetIsChopped true)
          (bind _returnvalue_4 (Game|SpawnActorfromClass "/Game/Tree/BP_ChoppedTree.BP_ChoppedTree_C" (Transformation|GetActorTransform) "AdjustIfPossibleButAlwaysSpawn" self 0))
          ;[1 0.8906 0] 나무를 쓰러뜨립니다
          (Physics|AddImpulseatLocation (Variables|/Script/Engine.StaticMeshActor|GetStaticMeshComponent _returnvalue_4) (* (* (LocalVariables|GetToProjectedHitPoint) -1.0) (Math|Float|MakeLiteralFloat 5e+04)) (+ (* (Math|Vector|GetUpVector (Variables|/Script/Engine.StaticMeshActor|GetStaticMeshComponent _returnvalue_4)) (.Z (Math|Vector|BreakVector (.Max (Components|StaticMesh|GetLocalBounds (Variables|/Script/Engine.StaticMeshActor|GetStaticMeshComponent _returnvalue_4)))))) (Transformation|GetWorldLocation (Variables|/Script/Engine.StaticMeshActor|GetStaticMeshComponent _returnvalue_4)) (* (LocalVariables|GetToProjectedHitPoint) 5e+01)) "None"))
        (else
          (Utilities|FlowControl|Sequence
            (:then_0
              (LocalVariables|SetHitIndex (CallFunction|ClampIndex (Math|Float|Round (Math|Float|MapRangeClamped (CallFunction|GetSignedDegreeBetweenVectors (Math|Vector|GetForwardVector (Variables|Default|GetChopPlane)) (LocalVariables|GetToProjectedHitPoint) (Math|Vector|GetUpVector (Variables|Default|GetChopPlane))) -1.8e+02 1.8e+02 0.0 (Math|Conversions|ToFloat(Integer) (Variables|Default|GetChopMapLength))))))
              (Class|KismetMathLibrary|LinearColorSetRandomHue (LocalVariables|GetRandomColor))
              (for _index (range (- (LocalVariables|GetHitIndex) _returnvalue_3) (+ (LocalVariables|GetHitIndex) _returnvalue_3))
                (Utilities|Array|SetArrayElem (Variables|Default|GetChopMap) (CallFunction|ClampIndex _index) (Math|Float|Clamp(Float) (+ (Utilities|Array|Get(acopy) (Variables|Default|GetChopMap) (CallFunction|ClampIndex _index)) (CallFunction|GetAttanuatedDamage (LocalVariables|GetHitIndex) (CallFunction|ClampIndex _index) 0.25))))))
            (:then_1
              (for (_array_element _array_index) (Variables|Default|GetChopMap)
                (bind (_canvas _size _context) (Rendering|BeginDrawCanvastoRenderTarget (Variables|Default|GetChopMapTexture)))
                (Class|Canvas|DrawLine _canvas (Math|Vector2D|MakeVector2D (- (Math|Conversions|ToFloat(Integer) _array_index) 0.5) 0.0) (Math|Vector2D|MakeVector2D (+ (Math|Conversions|ToFloat(Integer) _array_index) 0.5) 1.0) 1.0 (Math|Color|MakeColor _array_element _array_element _array_element))
                (Rendering|EndDrawCanvastoRenderTarget _context)))))))))

(fn Update(MainStaticMesh)
  (params (Show :type Boolean))
  (Rendering|SetVisibility (Variables|Default|GetStaticMeshComponent) Show false)
  (Collision|SetCollisionEnabled (Variables|Default|GetStaticMeshComponent) (select Show "QueryAndPhysics" "NoCollision")))

(fn Update(BottomStaticMesh)
  (params (Show :type Boolean))
  (Rendering|SetVisibility (Variables|Default|GetBottomStaticMesh) Show false)
  (Collision|SetCollisionEnabled (Variables|Default|GetBottomStaticMesh) (select Show "QueryAndPhysics" "NoCollision")))

(fn IsChoppedEnough
  (LocalVariables|SetChoppedCount 0)
  (for _array_element (Variables|Default|GetChopMap)
    (if (>= _array_element 1.0)
      (Math|Integer|IncrementInt (LocalVariables|GetChoppedCount))))
  ;[1 0 0.6562] 충분히 잘렸나?
  (return (|({3FEE8C54-4896-F03E-9136-A59024D738EA}>=({EBCEE680-45A4-6C14-DFBA-FF9408E3DA09}*0.250000)))))

(fn Initialize(BottomStaticMesh)
  (Rendering|Material|SetMaterial (Variables|Default|GetBottomStaticMesh) 0 (Variables|Default|GetTreeDMI)))